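; Grindable spline prop, apparently a parent class, that tells ThirdPersonCharacter when it can grind.
; Construction script builds spline meshes along the spline, raised above its points.
; While the player overlaps SphereCollision, Tick compares capsule distance to the closest spline point, setting CanGrind within DistanceToStartGrind; leaving clears it.
; BeginPlay passes its class to the character; debug prints and spheres remain, and FindClosestPointToCharacter is disconnected.
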(event `self.ReceiveBeginPlay`
  (bind _returnvalue (`GameplayStatics.GetObjectClass` self))
  (bind _asthird_person_character (cast `/Game/Blueprints/Characters/ThirdPersonCharacter` (`GameplayStatics.GetPlayerCharacter` 0)))
  (bind _output_get (set `self.Character` _asthird_person_character))
  (set `/Game/Blueprints/Characters/ThirdPersonCharacter.GrindPropReference` _returnvalue _output_get)
  (`KismetSystemLibrary.PrintString` (`KismetSystemLibrary.GetClassDisplayName` _returnvalue)))

(event `self.ReceiveTick`
  (params (DeltaSeconds :type "Float (single-precision)"))
  (if (stale `self.SphereCollision.OnComponentBeginOverlap` _output_get)
    (`self.CanGrind?`)))

(event `self.SphereCollision.OnComponentBeginOverlap`
  (params (OverlappedComponent :type "PrimitiveComponent Object Reference") (OtherActor :type "Actor Object Reference") (OtherComp :type "PrimitiveComponent Object Reference") (OtherBodyIndex :type Integer) (bFromSweep :type Boolean) (SweepResult :type "HitResult Structure (by ref)"))
  (bind _asthird_person_character (cast `/Game/Blueprints/Characters/ThirdPersonCharacter` OtherActor))
  (bind _output_get (set `self.IsPlayerColliding` true)))

(event `self.SphereCollision.OnComponentEndOverlap`
  (params (OverlappedComponent :type "PrimitiveComponent Object Reference") (OtherActor :type "Actor Object Reference") (OtherComp :type "PrimitiveComponent Object Reference") (OtherBodyIndex :type Integer))
  (bind _asthird_person_character (cast `/Game/Blueprints/Characters/ThirdPersonCharacter` OtherActor))
  (set `self.IsPlayerColliding` false)
  (set `/Game/Blueprints/Characters/ThirdPersonCharacter.CanGrind` false _asthird_person_character))

(fn `CanGrind?`
  (bind _asthird_person_character (cast `/Game/Blueprints/Characters/ThirdPersonCharacter` (`GameplayStatics.GetPlayerCharacter` 0)))
  (bind _returnvalue (`SceneComponent.K2_GetComponentLocation` (`Character.CapsuleComponent` _asthird_person_character)))
  (bind _returnvalue_2 (`SplineComponent.FindLocationClosestToWorldLocation` (`self.Spline`) _returnvalue "World"))
  (bind _returnvalue_3 (`KismetMathLibrary.Vector_Distance` _returnvalue_2 _returnvalue))
  (`KismetSystemLibrary.PrintString` (`KismetStringLibrary.Conv_DoubleToString` _returnvalue_3))
  (`KismetSystemLibrary.DrawDebugSphere` _returnvalue_2 10.0 12 (struct :`R` 1.0 :`G` 1.0 :`B` 1.0 :`A` 1.0) 2.0)
  (if (<= _returnvalue_3 (`self.DistanceToStartGrind`))
    (`/Engine/EditorBlueprintResources/StandardMacros.DoOnce` false
      (:`Completed`
        (set `/Game/Blueprints/Characters/ThirdPersonCharacter.CanGrind` true _asthird_person_character)
        (return)))))

(fn `FindClosestPointToCharacter`
  (returns (Output_Get :type "Vector Structure")))

(fn `UserConstructionScript`
  (bind _spline (`self.Spline`))
  (bind _spline_2 (`self.Spline`))
  (for _index (range (`SplineComponent.GetNumberOfSplinePoints` (`self.Spline`)))
    (bind _returnvalue (`AddComponent|NODE_AddSplineMeshComponent-0`))
    (`SplineMeshComponent.SetForwardAxis` _returnvalue "X" true)
    (bind (_returnvalue_x _returnvalue_y _returnvalue_z) (`KismetMathLibrary.BreakVector` (`SplineComponent.GetLocationAtSplinePoint` _spline _index "Local")))
    (bind _returnvalue_2 (+ _index 1))
    (bind (_returnvalue_x_2 _returnvalue_y_2 _returnvalue_z_2) (`KismetMathLibrary.BreakVector` (`SplineComponent.GetLocationAtSplinePoint` _spline_2 _returnvalue_2 "Local")))
    (`SplineMeshComponent.SetStartAndEnd` _returnvalue (`KismetMathLibrary.MakeVector` _returnvalue_x _returnvalue_y (+ _returnvalue_z 50.0)) (`SplineComponent.GetTangentAtSplinePoint` _spline _index "Local") (`KismetMathLibrary.MakeVector` _returnvalue_x_2 _returnvalue_y_2 (+ _returnvalue_z_2 50.0)) (`SplineComponent.GetTangentAtSplinePoint` _spline_2 _returnvalue_2 "Local") true)))